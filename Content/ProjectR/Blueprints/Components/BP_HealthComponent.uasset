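; Health component that tracks current health against a maximum and flags death.
; TakeDamage and Heal events adjust Health, clamped between zero and MaxHealth.
; Damage that leaves Health at zero calls HandleDeath, which sets IsDead and only prints a player death message.
; Neither event checks IsDead, so death handling can repeat and healing can raise Health afterward without clearing the flag.
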(event `TakeDamage`
  (params (`Damage Amount` :type "Float (double-precision)"))
  ;[1 1 1] Take Damage Function
  (set `self.Health` (`KismetMathLibrary.FClamp` (- (`self.Health`) `Damage Amount`) 0.0 (`self.MaxHealth`)))
  (if (<= (`self.Health`) 0.0)
    (`self.HandleDeath`)))

(event `Heal`
  (params (` HealAmount ` :type "Float (double-precision)"))
  ;[1 1 1] Healing Function
  (set `self.Health` (`KismetMathLibrary.FClamp` (+ (`self.Health`) ` HealAmount `) 0.0 (`self.MaxHealth`))))

(event `HandleDeath`
  (set `self.isDead?` true)
  (`KismetSystemLibrary.PrintString` "Player Died"))