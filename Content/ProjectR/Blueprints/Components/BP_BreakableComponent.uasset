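; Breakable component that physically breaks apart an object and drives a dissolve material parameter.
; BreakObject enables physics on every static mesh of MeshToBreak's owner, ignoring only pawns, and requests a looping dissolve timer.
; UpdateDissolveEffect sets DissolveAmount from frame delta over DissolveDuration, without accumulating.
; The completion check that clears the timer and destroys the owner runs only once, within BreakObject.
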(event `BreakObject`
  (params (Alpha :type "Float (double-precision)"))
  (for _array_element (`Actor.K2_GetComponentsByClass` (`self.GetOwner` (`self.MeshToBreak`)) "/Script/Engine.StaticMeshComponent")
    (bind _asstatic_mesh_component (cast `StaticMeshComponent` _array_element))
    (`PrimitiveComponent.SetSimulatePhysics` _asstatic_mesh_component true)
    (`PrimitiveComponent.SetCollisionEnabled` _asstatic_mesh_component "QueryAndPhysics")
    (`PrimitiveComponent.SetCollisionProfileName` _asstatic_mesh_component "IgnoreOnlyPawn" true))
  (`KismetSystemLibrary.K2_SetTimer` null "UpdateDissolveEffect" 0.0 true)
  (bind _returnvalue (`MaterialInstanceDynamic.K2_GetScalarParameterValue` (`self.DynamicMaterial`) "DissolveAmount"))
  (`KismetSystemLibrary.PrintString` (`KismetStringLibrary.Conv_DoubleToString` _returnvalue))
  (if (>= _returnvalue 1.0)
    (`KismetSystemLibrary.K2_ClearTimer` null "UpdateDissolveEffect")
    (`Actor.K2_DestroyActor` (`self.GetOwner`))))

(fn `UpdateDissolveEffect`
  (bind _output_get (set `self.CurrentDissolveAmount ` (`KismetMathLibrary.FClamp` (/ (`GameplayStatics.GetWorldDeltaSeconds`) (`self.DissolveDuration`)))))
  (`MaterialInstanceDynamic.SetScalarParameterValue` (`self.DynamicMaterial`) "DissolveAmount" _output_get))