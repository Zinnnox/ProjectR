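; BP_InteractableObject is a world object the first-person player can approach and inspect through an item preview.
; Its collision trigger registers it as the player's current interactable and shows the HUD interaction prompt, undoing both on exit.
; Interact plays a sound, spawns a BP_ItemPreviewScene fed the object's static mesh, adds a preview widget and hides other HUD elements.
; StopInteract, also called on leaving the trigger, closes that preview, with a flag blocking repeat interactions.
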(event `self.CollisionTrigger.OnComponentBeginOverlap`
  (params (OverlappedComponent :type "PrimitiveComponent Object Reference") (OtherActor :type "Actor Object Reference") (OtherComp :type "PrimitiveComponent Object Reference") (OtherBodyIndex :type Integer) (bFromSweep :type Boolean) (SweepResult :type "HitResult Structure (by ref)"))
  ;[1 1 1] Trigger Pickup Message
  (bind _asbp_first_person_character (cast `/Game/FirstPerson/Blueprints/BP_FirstPersonCharacter` OtherActor))
  (bind _output_get (set `self.PlayerRef` _asbp_first_person_character))
  (bind _playerhudref (`/Game/FirstPerson/Blueprints/BP_FirstPersonCharacter.PlayerHUDRef` _output_get))
  (set `self.HUDRef` _playerhudref)
  (`/Game/FirstPerson/Blueprints/BP_FirstPersonCharacter.SetCurrentInteractable` _output_get self)
  (bind _output_get_2 (set `self.InteractionWidgetInstance` (`/Game/ProjectR/Blueprints/UI/InGame/WB_PlayerHUD.InteractionPrompt` _playerhudref)))
  (`/Game/ProjectR/Blueprints/UI/BPI_UIManager.ShowSpecificUI` (`self.HUDRef`) _output_get_2)
  (set `/Game/FirstPerson/Blueprints/BP_FirstPersonCharacter.bIsPreviewActive` true (`self.PlayerRef`)))

(event `self.CollisionTrigger.OnComponentEndOverlap`
  (params (OverlappedComponent :type "PrimitiveComponent Object Reference") (OtherActor :type "Actor Object Reference") (OtherComp :type "PrimitiveComponent Object Reference") (OtherBodyIndex :type Integer))
  (bind _interactionwidgetinstance (`self.InteractionWidgetInstance`))
  ;[1 1 1] Remove pick up message from screen when too far
  (bind _asbp_first_person_character (cast `/Game/FirstPerson/Blueprints/BP_FirstPersonCharacter` OtherActor))
  (`self.StopInteract`)
  (`/Game/FirstPerson/Blueprints/BP_FirstPersonCharacter.ClearCurrentInteractable` _asbp_first_person_character)
  (`/Engine/EditorBlueprintResources/StandardMacros.IsValid` _interactionwidgetinstance
    (:`Is Valid`
      (`/Game/ProjectR/Blueprints/UI/BPI_UIManager.HideSpecificUI` (`self.HUDRef`) _interactionwidgetinstance)
      (set `self.InteractionWidgetInstance` null)
      (set `/Game/FirstPerson/Blueprints/BP_FirstPersonCharacter.bIsPreviewActive` false (`self.PlayerRef`))
      (set `self.PreviewWidgetInstance` null)
      (set `self.PlayerRef` null))))

(event `Interact`
  (if (not (`self.hasInteractedYet`))
    (set `self.hasInteractedYet` true)
    (`GameplayStatics.PlaySoundAtLocation` (`self.InteractSound`) (`self.K2_GetActorLocation`) (struct) 1.0 1.0 0.0 null null null null)
    (bind _returnvalue (`|SpawnActorFromClass` "/Game/ProjectR/Blueprints/BP_ItemPreviewScene.BP_ItemPreviewScene_C" (`self.PreviewSpawnTransform`) "Undefined" "MultiplyWithRoot" null null))
    (bind _output_get (set `self.SpawnedPreviewActor` _returnvalue))
    (`/Game/ProjectR/Blueprints/BP_ItemPreviewScene.InitPreview` _output_get (`StaticMeshComponent.StaticMesh` (`self.SM_Object`)))
    (bind _returnvalue_2 (`|CreateWidget` "/Game/ProjectR/Blueprints/UI/InGame/WB_ItemPreviewWidget.WB_ItemPreviewWidget_C"))
    (bind _output_get_2 (set `self.PreviewWidgetInstance` _returnvalue_2))
    (`UserWidget.AddToViewport` _output_get_2 0)
    (message `/Game/ProjectR/Blueprints/UI/BPI_UIManager.HideAllUIElements` (`self.HUDRef`))))

(event `StopInteract`
  (if (`self.hasInteractedYet`)
    (set `self.hasInteractedYet` false)
    (`/Game/ProjectR/Blueprints/BP_ItemPreviewScene.ClosePreview` (`self.SpawnedPreviewActor`))))

(fn `UserConstructionScript`)