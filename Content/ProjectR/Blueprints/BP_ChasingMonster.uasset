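; Enemy character that chases the first-person player and attacks at close range while gravity direction can change.
; Tick turns it toward the player on the plane of the player's up vector, moves it forward and attempts attacks.
; Hits damage the player's health component, start a cooldown and launch the monster backward.
; On the player's gravity switch, it pauses, adopts the new gravity after a delay, then rotates upright through a timeline lerp.
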(event `self.ReceiveBeginPlay`
  ;[1 1 1] Store Player reference
  (bind _asbp_first_person_character (cast `/Game/FirstPerson/Blueprints/BP_FirstPersonCharacter` (`GameplayStatics.GetPlayerCharacter` 0)))
  (set `self.PlayerActorRef` _asbp_first_person_character)
  (set `self.MonsterDownVector` (`CharacterMovementComponent.GetGravityDirection` (`self.CharacterMovement`)))
  (add `/Game/FirstPerson/Blueprints/BP_FirstPersonCharacter.OnSuccessfulGravitySwitch` (`self.PlayerActorRef`) (delegate `OnPlayerGravitySwitch`)))

(event `OnPlayerGravitySwitch`
  (`KismetSystemLibrary.PrintString` "PLAYER CHANGED GRAV")
  (set `self.Player'sNewGravity` (`/Game/FirstPerson/Blueprints/BP_FirstPersonCharacter.New Gravity Down Direction` (`self.PlayerActorRef`)))
  (set `self.IsFlippingGravity` true)
  (`KismetSystemLibrary.Delay` 1.5)
  (`self.FlipToGravity` (`self.Player'sNewGravity`)))

(event `self.ReceiveTick`
  (params (DeltaSeconds :type "Float (single-precision)"))
  (if (and (not (`self.IsFlippingGravity`)) (not (`/Game/ProjectR/Blueprints/Components/BP_HealthComponent.isPlayerDead?` (`/Game/FirstPerson/Blueprints/BP_FirstPersonCharacter.BP_HealthComponent` (`self.PlayerActorRef`)))))
    (`self.FollowPlayer`)
    (`self.TryAttack`)))

(event `ApplyDamage`
  (set `self.CanAttack` false)
  (`/Game/ProjectR/Blueprints/Components/BP_HealthComponent.TakeDamage` (`self.GetComponentByClass` (`self.PlayerActorRef`) "/Game/ProjectR/Blueprints/Components/BP_HealthComponent.BP_HealthComponent_C") (`self.DamageAmount`))
  (`KismetSystemLibrary.Delay` (`self.AttackCooldownTime`))
  (set `self.CanAttack` true))

(event `FlipToGravity`
  (params (NewMonsterGravityDirection :type "Vector Structure"))
  ;[1 1 1] Flip enemy gravity to match player with delay and upright alignment
  (bind _output_get (set `self.MonsterDownVector` NewMonsterGravityDirection))
  (set `self.MonsterUpVector` (* _output_get -1.0))
  (`KismetSystemLibrary.PrintString` (`KismetStringLibrary.BuildString_Vector` "New Gravity Direction FOR MONSTER: " "" _output_get))
  (bind _output_get_2 (set `self.DesiredRotation` (`self.GetRotatorToLookAtPlayer`)))
  (`KismetSystemLibrary.PrintString` (`KismetStringLibrary.Concat_StrStr` "NEW ROTATOR FOR MONSTER" (`KismetStringLibrary.Conv_RotatorToString` _output_get_2)))
  (`CharacterMovementComponent.SetGravityDirection` (`self.CharacterMovement`) (`self.Player'sNewGravity`))
  (`self.K2_SetActorLocation` (+ (`self.K2_GetActorLocation`) (* (`self.MonsterDownVector`) -5)))
  (bind (_direction _alphatrack) (`Timeline|Timeline` :`NewTime` 0.25 :!via `PlayFromStart`)
    (:`Update`
      (`self.K2_SetActorRotation` (`KismetMathLibrary.RLerp` (`self.K2_GetActorRotation`) (`self.DesiredRotation`) _alphatrack true)))
    (:`Finished`
      (set `self.IsFlippingGravity` false))))

(fn `FollowPlayer`
  (locals (Direction :type "Vector Structure"))
  ;[1 1 1] Move toward player using direction vector
  (`/Engine/EditorBlueprintResources/StandardMacros.IsValid` (`self.PlayerActorRef`)
    (:`Is Valid`
      (`self.AddMovementInput` (`self.GetActorForwardVector`) (`self.MoveSpeed`))
      (`self.K2_SetActorRotation` (`self.GetRotatorToLookAtPlayer`))
      (`KismetSystemLibrary.PrintString` "Chasing player!" :!enabledstate Disabled))))

(fn `Get Direction From Player`
  (returns (Direction :type "Vector Structure"))
  (locals (Direction :type "Vector Structure"))
  (return (- (`CharacterMovementComponent.GetLastUpdateLocation` (`self.CharacterMovement`)) (`CharacterMovementComponent.GetLastUpdateLocation` (`Character.CharacterMovement` (`self.PlayerActorRef`))))))

(fn `Get Direction To Player`
  (returns (Direction :type "Vector Structure"))
  (locals (Direction :type "Vector Structure"))
  (return (- (`CharacterMovementComponent.GetLastUpdateLocation` (`Character.CharacterMovement` (`self.PlayerActorRef`))) (`CharacterMovementComponent.GetLastUpdateLocation` (`self.CharacterMovement`)))))

(fn `GetRotatorToLookAtPlayer`
  (returns (ReturnValue :type "Rotator Structure"))
  (bind _direction (`self.Get Direction To Player`))
  (bind _newup (`/Game/FirstPerson/Blueprints/BP_FirstPersonCharacter.NewUp` (`self.PlayerActorRef`)))
  (return (`KismetMathLibrary.MakeRotFromXZ` (`KismetMathLibrary.Normal` (- _direction (* (`KismetMathLibrary.Dot_VectorVector` _direction _newup) _newup))) _newup)))

(fn `TryAttack`
  (locals (Distance :type "Float (double-precision)" :default 0.0))
  (`/Engine/EditorBlueprintResources/StandardMacros.IsValid` (`self.PlayerActorRef`)
    (:`Is Valid`
      (if (== (`self.CanAttack`) true)
        (set `local.Distance` (`KismetMathLibrary.Vector_Distance` (`CharacterMovementComponent.GetLastUpdateLocation` (`Character.CharacterMovement` (`self.PlayerActorRef`))) (`CharacterMovementComponent.GetLastUpdateLocation` (`self.CharacterMovement`))))
        (if (< (`local.Distance`) (`self.AttackRange`))
          (`self.ApplyDamage`)
          (`KismetSystemLibrary.PrintString` "ATTACK!")
          ;[1 1 1] Push monster away from player after hit to give escape window
          (`self.LaunchCharacter` (* (`KismetMathLibrary.Normal` (`self.Get Direction From Player`)) (`self.KnockbackAmount`)) true))))))

(fn `UserConstructionScript`)