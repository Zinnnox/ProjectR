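; Procedural level generator that chains a start room, random RoomPool snippets and an exit room that receives the next level to load.
; Each delayed spawn snaps its Entry-tagged component to the previous room's Exit by composing transforms, destroying and retrying if either is missing.
; The random pool index is bounded by the spawned room count, not pool size.
; GetComponentWithTag also spawns enemy triggers and destructible walls at tagged components on every lookup.
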(event `self.ReceiveBeginPlay`
  (if (`self.StartAtBeginPlay?`)
    (`KismetSystemLibrary.PrintString` "LevelGenerator STarts " :!enabledstate Disabled)
    (`self.StartGeneration`)))

(event `StartGeneration`
  ;[1 1 1] init level generation variables -- spawn first room
  (`KismetArrayLibrary.Array_Clear` (`self.SpawnedRooms`))
  (set `self.CurrentRoomIndex` 0)
  (bind _returnvalue (`|SpawnActorFromClass` (`self.StartSnippet`) (`self.GetTransform`) "Undefined" "MultiplyWithRoot" null null))
  (bind _output_get (set `self.LastSpawnedRoom` _returnvalue))
  (`KismetArrayLibrary.Array_Add` (`self.SpawnedRooms`) _output_get)
  (`self.SpawnNextRoom`))

(event `SpawnNextRoom`
  (bind _returnvalue (`KismetArrayLibrary.Array_Length` (`self.SpawnedRooms`)))
  (bind _output (`|GetArrayItem` (`self.RoomPool`) (`KismetMathLibrary.RandomIntegerInRange` 0 (- _returnvalue 1))))
  (if (>= _returnvalue (`self.NumRoomsToSpawn`)) :!label _label
    ;[1 1 1] final room
    (if (not (`self.FinishedGeneration?`))
      (`KismetSystemLibrary.Delay` 0.2)
      (bind _returnvalue_2 (`|SpawnActorFromClass` (`self.ExitSnippet`) (`KismetMathLibrary.MakeTransform` (0.0 0.0 0.0)) "Undefined" "MultiplyWithRoot" null null))
      (bind _asexit_room (cast `/Game/Maps/room_snippets/ExitRoom` _returnvalue_2))
      (set `/Game/Maps/room_snippets/ExitRoom.NextLevelToLoad` (`self.Next Level to Load`) _asexit_room)
      (if (`KismetSystemLibrary.IsValid` _returnvalue_2)
        (bind _output_get (set `self.NewestSpawnedRoom` _returnvalue_2))
        (`KismetArrayLibrary.Array_Add` (`self.SpawnedRooms`) _output_get)
        (`self.AlignRoomToPrevious` (`self.NewestSpawnedRoom`) (`self.LastSpawnedRoom`))
        (set `self.FinishedGeneration?` true)
        (`KismetSystemLibrary.PrintString` "rooms spawned equal desired number" :!enabledstate Disabled)))
    (else
      ;[1 1 1] for each room
      (if (`KismetSystemLibrary.IsValidClass` _output)
        (`KismetSystemLibrary.Delay` 0.2)
        (bind _returnvalue_3 (`|SpawnActorFromClass` _output (`KismetMathLibrary.MakeTransform` (0.0 0.0 0.0)) "Undefined" "MultiplyWithRoot" null null))
        (if (`KismetSystemLibrary.IsValid` _returnvalue_3)
          (bind _output_get_2 (set `self.NewestSpawnedRoom` _returnvalue_3))
          (`KismetArrayLibrary.Array_Add` (`self.SpawnedRooms`) _output_get_2)
          (`self.AlignRoomToPrevious` (`self.NewestSpawnedRoom`) (`self.LastSpawnedRoom`))
          (else
            (`self.SpawnNextRoom`)))
        (else
          (goto _label))))))

(event `AlignRoomToPrevious`
  (params (`New Room` :type "Actor Object Reference") (`Last Room` :type "Actor Object Reference"))
  (set `self.EntryComponent` (`self.GetComponentWithTag` `New Room` "Entry"))
  (set `self.ExitComponent` (`self.GetComponentWithTag` `Last Room` "Exit"))
  (if (or (== (`self.ExitComponent`) null) (== (`self.EntryComponent`) null))
    ;[1 1 1] retry if necessary
    (`KismetSystemLibrary.PrintString` (`KismetStringLibrary.Concat_StrStr` "SKIPPING ALIGNMENT -- " "Missing entry or exit on " (`KismetSystemLibrary.GetDisplayName` `New Room`)) :!enabledstate Disabled)
    (`self.K2_DestroyActor` `New Room`)
    (`KismetArrayLibrary.Array_RemoveItem` (`self.SpawnedRooms`) `New Room`)
    (`self.SpawnNextRoom`)
    (else
      ;[1 1 1] align to previous spawned room - then spawn next one
      (`self.K2_SetActorTransform` (`self.NewestSpawnedRoom`) (`KismetMathLibrary.ComposeTransforms` (`KismetMathLibrary.InvertTransform` (`SceneComponent.K2_GetComponentToWorld` (`self.EntryComponent`))) (`SceneComponent.K2_GetComponentToWorld` (`self.ExitComponent`))) false true)
      (set `self.LastSpawnedRoom` (`self.NewestSpawnedRoom`))
      (`KismetSystemLibrary.DelayUntilNextTick`)
      (`self.SpawnNextRoom`))))

(fn `GetComponentWithTag`
  (params (Actor :type "Actor Object Reference") (Tag :type Name))
  (returns (Component :type "SceneComponent Object Reference"))
  (locals (ActorInput :type "Actor Object Reference") (CurrentSceneComp :type "SceneComponent Object Reference"))
  (bind _returnvalue (`KismetSystemLibrary.GetDisplayName` Actor))
  (bind _returnvalue_2 (`self.GetComponentsByTag` (`local.ActorInput`) "/Script/Engine.SceneComponent" Tag))
  (bind _returnvalue_3 (`SceneComponent.K2_GetComponentToWorld` (`local.CurrentSceneComp`)))
  (bind _output (`|GetArrayItem` _returnvalue_2))
  (set `local.ActorInput` Actor)
  (for _array_element (`self.K2_GetComponentsByClass` (`local.ActorInput`) "/Script/Engine.SceneComponent")
    (set `local.CurrentSceneComp` _array_element)
    (for _array_element_2 (`ActorComponent.ComponentTags` (`local.CurrentSceneComp`))
      (switch `name` _array_element_2
        (:`EnemySpawnTrigger`
          (`KismetSystemLibrary.PrintString` (`KismetSystemLibrary.GetDisplayName` (`local.CurrentSceneComp`)))
          (bind _returnvalue_4 (`|SpawnActorFromClass` "/Game/Maps/room_snippets/BP_EnemySpawnTrigger.BP_EnemySpawnTrigger_C" _returnvalue_3 "Undefined" "MultiplyWithRoot" null (`local.ActorInput`) 0.5 null))
          (`KismetSystemLibrary.PrintString` (`KismetSystemLibrary.GetDisplayName` (`/Game/Maps/room_snippets/BP_EnemySpawnTrigger.RoomOwner` _returnvalue_4))))
        (:`DWSpawnPoint`
          (`|SpawnActorFromClass` "/Game/ProjectR/Blueprints/BP_DestructibleWall.BP_DestructibleWall_C" _returnvalue_3 "Undefined" "MultiplyWithRoot" null null)))))
  (if (and (> (`KismetArrayLibrary.Array_Length` (`self.RoomPool`)) 0) (> (`KismetArrayLibrary.Array_Length` _returnvalue_2) 0))
    (if (`KismetSystemLibrary.IsValid` _output)
      (`KismetSystemLibrary.PrintString` (`KismetStringLibrary.Concat_StrStr` "This actor " _returnvalue "has component " (`KismetSystemLibrary.GetDisplayName` _output)) :!enabledstate Disabled)
      (return _output)
      (else
        (`KismetSystemLibrary.PrintString` (`KismetStringLibrary.Concat_StrStr` "THIS ACTOR: " _returnvalue "DOES NOT HAVE A COMPONENT with TAG: " (`KismetStringLibrary.Conv_NameToString` Tag)) :!enabledstate Disabled)
        (return null)))))

(fn `UserConstructionScript`)