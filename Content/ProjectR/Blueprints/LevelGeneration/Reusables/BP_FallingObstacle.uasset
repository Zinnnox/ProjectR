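; BP_FallingObstacle is a level-generation obstacle that drops and damages the first-person player.
; A two-second delay after BeginPlay, marked as a stand-in for a room trigger, enables gravity on VisualMesh and sets HasFallen.
; BoxTrigger overlaps after that damage the player's health component and break the mesh through BPBreakableComponent.
; The player reference is cached on first cast, so later overlaps skip the actor check.
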(event `self.ReceiveBeginPlay`
  (`KismetSystemLibrary.Delay` 2.0) ; replace with room trigger
  (`PrimitiveComponent.SetEnableGravity` (`self.VisualMesh`) true)
  (set `self.HasFallen?` true))

(event `self.BoxTrigger.OnComponentBeginOverlap`
  (params (OverlappedComponent :type "PrimitiveComponent Object Reference") (OtherActor :type "Actor Object Reference") (OtherComp :type "PrimitiveComponent Object Reference") (OtherBodyIndex :type Integer) (bFromSweep :type Boolean) (SweepResult :type "HitResult Structure (by ref)"))
  (if (`self.HasFallen?`)
    (if (not (`KismetSystemLibrary.IsValid` (`self.PlayerRef`)))
      (bind _asbp_first_person_character (cast `/Game/FirstPerson/Blueprints/BP_FirstPersonCharacter` OtherActor))
      (bind _output_get (set `self.PlayerRef` _asbp_first_person_character)))
    (`/Game/ProjectR/Blueprints/Components/BP_HealthComponent.TakeDamage` (`/Game/FirstPerson/Blueprints/BP_FirstPersonCharacter.BP_HealthComponent` _output_get) (`self.DamageAmount`))
    (set `/Game/ProjectR/Blueprints/Components/BP_BreakableComponent.MeshToBreak` (`self.VisualMesh`) (`self.BP_BreakableComponent`))
    (`/Game/ProjectR/Blueprints/Components/BP_BreakableComponent.BreakObject` (`self.BP_BreakableComponent`))))

(fn `UserConstructionScript`)