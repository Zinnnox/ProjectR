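; Moving platform that travels back and forth along a spline, pausing at each end.
; Tick advances a running time, scales it by move speed and folds it with a remainder over twice the spline length into a ping-pong distance.
; The mesh takes the spline's world location and rotation at that distance.
; Near either end, a delay halts movement and the time accumulation for the pause duration.
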(event `self.ReceiveBeginPlay`
  (set `self.SplineLength` (`SplineComponent.GetSplineLength` (`self.Path`))))

(event `self.ReceiveTick`
  (params (DeltaSeconds :type "Float (single-precision)"))
  (if (not (`self.IsPaused?`))
    (`self.Move Platform` DeltaSeconds)))

(event `Move Platform`
  (params (DeltaSeconds :type "Float (double-precision)"))
  (bind _path (`self.Path`))
  (bind _effectivedistance (`self.EffectiveDistance`))
  (bind _returnvalue (* (`self.SplineLength`) 2.0))
  (bind _output_get (set `self.RunningTime` (+ (`self.RunningTime`) DeltaSeconds)))
  (bind _output_get_2 (set `self.DeltaDistance` (* _output_get (`self.MoveSpeed`))))
  (bind _remainder (`KismetMathLibrary.FMod` _output_get_2 _returnvalue))
  (if (> _remainder (`self.SplineLength`))
    (set `self.EffectiveDistance` (- _returnvalue _remainder))
    (else
      (set `self.EffectiveDistance` _remainder)))
  (if (and (or (`KismetMathLibrary.NearlyEqual_FloatFloat` (`self.EffectiveDistance`) 0.0 1.0) (`KismetMathLibrary.NearlyEqual_FloatFloat` (`self.EffectiveDistance`) (`self.SplineLength`) 1.0)) (== (`self.JustPaused?`) false))
    (`self.PauseAtEnds`))
  (`SceneComponent.K2_SetWorldLocationAndRotation` (`self.PlatformMesh`) (`SplineComponent.GetLocationAtDistanceAlongSpline` _path _effectivedistance "World") (`SplineComponent.GetRotationAtDistanceAlongSpline` _path _effectivedistance "World") false false))

(event `PauseAtEnds`
  (`KismetSystemLibrary.PrintString` "Reached end")
  (set `self.IsPaused?` true)
  (set `self.JustPaused?` true)
  (`KismetSystemLibrary.Delay` (`self.PauseDuration`))
  (set `self.IsPaused?` false)
  (set `self.JustPaused?` false))

(fn `UserConstructionScript`)