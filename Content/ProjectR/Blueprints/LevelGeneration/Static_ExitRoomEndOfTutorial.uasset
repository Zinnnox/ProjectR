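; Tutorial exit room actor with a porta-potty door that loads the next level when the player uses it.
; An overlap trigger tracks the player, and Tick fires the interaction once when E is held nearby and the door is still closed.
; Interacting swings the door open on a timeline, disables player input, fades to black via the reused death screen widget, then opens the configured level after a delay.
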(event `self.ReceiveBeginPlay`
  (`self.EnableInput` (`GameplayStatics.GetPlayerController` 0)))

(event `Key|E`
  (params (Key :type "Key Structure"))
  (:`Pressed`
    (set `self.Is E Key Pressed` true))
  (:`Released`
    (set `self.Is E Key Pressed` false)))

(event `self.ReceiveTick`
  (params (DeltaSeconds :type "Float (single-precision)"))
  (if (and (== (`self.IsDoorOpen?`) false) (`self.IsPlayerNear?`) (`self.Is E Key Pressed`))
    (`self.InteractWithDoor`)))

(event `self.DoorTrigger.OnComponentBeginOverlap`
  (params (OverlappedComponent :type "PrimitiveComponent Object Reference") (OtherActor :type "Actor Object Reference") (OtherComp :type "PrimitiveComponent Object Reference") (OtherBodyIndex :type Integer) (bFromSweep :type Boolean) (SweepResult :type "HitResult Structure (by ref)"))
  (bind _returnvalue (`GameplayStatics.GetPlayerCharacter` 0))
  (bind _asbp_first_person_character (cast `/Game/FirstPerson/Blueprints/BP_FirstPersonCharacter` OtherActor))
  (if (== _asbp_first_person_character _returnvalue)
    (set `self.PlayerCharacterRef` _returnvalue)
    (set `self.IsPlayerNear?` true)))

(event `self.DoorTrigger.OnComponentEndOverlap`
  (params (OverlappedComponent :type "PrimitiveComponent Object Reference") (OtherActor :type "Actor Object Reference") (OtherComp :type "PrimitiveComponent Object Reference") (OtherBodyIndex :type Integer))
  (if (`self.IsPlayerNear?`)
    (set `self.IsPlayerNear?` false)))

(event `InteractWithDoor`
  (set `self.IsDoorOpen?` true)
  (`self.OpenAnimation`)
  (`self.DisableInput` (`self.PlayerCharacterRef`) (`GameplayStatics.GetPlayerController` 0))
  (`self.BlackFadeScreenTransition`)
  (`KismetSystemLibrary.Delay` 4.0)
  (`GameplayStatics.OpenLevelBySoftObjectPtr` (`self.NextLevelToLoad`)))

(event `OpenAnimation`
  (bind (_direction _doorrotation) (`Timeline|OpenDoorTimeline` :!via `PlayFromStart`)
    (:`Update`
      (`KismetSystemLibrary.PrintString` (`KismetStringLibrary.Conv_DoubleToString` _doorrotation))
      (`SceneComponent.K2_SetRelativeRotation` (`self.SM_Portapotty_Door`) (`KismetMathLibrary.MakeRotator` 0.0 0.0 _doorrotation) false false))))

(fn `UserConstructionScript`)