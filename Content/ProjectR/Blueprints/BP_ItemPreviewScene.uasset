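; Item preview scene actor that shows a single item mesh spinning in front of a scene capture component.
; InitPreview swaps in the given mesh and restricts the capture to that component, while Tick yaws it at RotationSpeed.
; ClosePreview closes the preview widget on the BP_InteractableObject found by class, then attempts to restore the HUD through a first-person character cast.
; Its DestroyActor node is unconnected, so the scene never destroys itself.
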(event `self.ReceiveTick`
  (params (DeltaSeconds :type "Float (single-precision)"))
  (`SceneComponent.K2_AddRelativeRotation` (`self.SM_PreviewItem`) (`KismetMathLibrary.MakeRotator` 0.0 0.0 (* DeltaSeconds (`self.RotationSpeed`))) false false))

(event `InitPreview`
  (params (NewMesh :type "StaticMesh Object Reference"))
  (`StaticMeshComponent.SetStaticMesh` (`self.SM_PreviewItem`) NewMesh)
  (`SceneCaptureComponent.ShowOnlyComponent` (`self.SC_Capture`) (`self.SM_PreviewItem`)))

(event `ClosePreview`
  (bind _returnvalue (`GameplayStatics.GetActorOfClass` "/Game/ProjectR/Blueprints/BP_InteractableObject.BP_InteractableObject_C"))
  (`/Game/ProjectR/Blueprints/UI/InGame/WB_ItemPreviewWidget.CloseWidgetPreview` (`/Game/ProjectR/Blueprints/BP_InteractableObject.PreviewWidgetInstance` _returnvalue))
  (bind _asbp_first_person_character (cast `/Game/FirstPerson/Blueprints/BP_FirstPersonCharacter` (`self.GetParentActor` (`GameplayStatics.GetPlayerController` 0))))
  (message `/Game/ProjectR/Blueprints/UI/BPI_UIManager.ShowAllUIElements` (`/Game/FirstPerson/Blueprints/BP_FirstPersonCharacter.PlayerHUDRef` _asbp_first_person_character)))

(fn `UserConstructionScript`)