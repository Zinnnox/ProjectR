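; BP_ChasingGod is an enemy that feeds player detection to the blackboard of its AIC_ChasingGodController.
; On BeginPlay it gathers TargetPoints tagged PatrolPoint and caches that blackboard.
; DetectionSphere overlap with BP_FirstPersonCharacter sets CanSeePlayer and PlayerActor; any end overlap clears CanSeePlayer, without checking the actor.
; SetNextPatrolPoint is empty, and the logic that cycles patrol points into TargetLocation is disconnected, so it never runs.
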(event `self.ReceiveBeginPlay`
  (bind _outactors (`GameplayStatics.GetAllActorsOfClassWithTag` "/Script/Engine.TargetPoint" "PatrolPoint"))
  (set `self.PatrolPoints` _outactors)
  (bind _asaic_chasing_god_controller (cast `/Game/ProjectR/Blueprints/Enemy/ChasingGod/AIC_ChasingGodController` (`AIBlueprintHelperLibrary.GetAIController` self)))
  (set `self.Blackboard Comp` (`/Game/ProjectR/Blueprints/Enemy/ChasingGod/AIC_ChasingGodController.BlackboardComp` _asaic_chasing_god_controller)))

(event `self.DetectionSphere.OnComponentBeginOverlap`
  (params (OverlappedComponent :type "PrimitiveComponent Object Reference") (OtherActor :type "Actor Object Reference") (OtherComp :type "PrimitiveComponent Object Reference") (OtherBodyIndex :type Integer) (bFromSweep :type Boolean) (SweepResult :type "HitResult Structure (by ref)"))
  (bind _blackboard_comp (`self.Blackboard Comp`))
  (bind _asbp_first_person_character (cast `/Game/FirstPerson/Blueprints/BP_FirstPersonCharacter` OtherActor))
  (set `self.PlayerActor` _asbp_first_person_character)
  (`BlackboardComponent.SetValueAsBool` _blackboard_comp "CanSeePlayer" true)
  (`BlackboardComponent.SetValueAsObject` _blackboard_comp "PlayerActor" (`self.PlayerActor`)))

(event `self.DetectionSphere.OnComponentEndOverlap`
  (params (OverlappedComponent :type "PrimitiveComponent Object Reference") (OtherActor :type "Actor Object Reference") (OtherComp :type "PrimitiveComponent Object Reference") (OtherBodyIndex :type Integer))
  (`BlackboardComponent.SetValueAsBool` (`self.Blackboard Comp`) "CanSeePlayer" false))

(event `SetNextPatrolPoint`)

(fn `UserConstructionScript`)