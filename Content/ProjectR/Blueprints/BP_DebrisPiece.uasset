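; BP_DebrisPiece is a short-lived debris actor that gets launched on spawn, then fades out and destroys itself.
; BeginPlay puts a dynamic fence-debris dissolve material on SMDebris and applies a random velocity-change impulse, equal on all three axes.
; Tick accumulates time while IsFading is false, driving the FadeAmount parameter from 0 to 1 over FadeDuration before destroying the actor.
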(event `self.ReceiveBeginPlay`
  (bind _sm_debris (`self.SM_Debris`))
  (bind _returnvalue (`PrimitiveComponent.CreateDynamicMaterialInstance` _sm_debris 0 "/Game/ProjectR/Materials/Instances/MI_Dissolve_FenceDebris.MI_Dissolve_FenceDebris" "None"))
  (bind _output_get (set `self.DynamicMat` _returnvalue))
  (`PrimitiveComponent.SetMaterial` _sm_debris 0 _output_get)
  (`PrimitiveComponent.AddImpulse` (`self.SM_Debris`) (`KismetMathLibrary.Conv_DoubleToVector` (`KismetMathLibrary.RandomFloatInRange` 0.0 250.0)) "None" true))

(event `self.ReceiveTick`
  (params (DeltaSeconds :type "Float (single-precision)"))
  (if (not (`self.IsFading`))
    (bind _output_get (set `self.CurrentFadeTime` (+ DeltaSeconds (`self.CurrentFadeTime`))))
    (`KismetSystemLibrary.PrintString` (`KismetStringLibrary.Conv_DoubleToString` _output_get) :!enabledstate Disabled)
    (bind _returnvalue (`KismetMathLibrary.FClamp` (/ _output_get (`self.FadeDuration`))))
    (`KismetSystemLibrary.PrintString` (`KismetStringLibrary.Conv_DoubleToString` _returnvalue) :!enabledstate Disabled)
    (`MaterialInstanceDynamic.SetScalarParameterValue` (`self.DynamicMat`) "FadeAmount" _returnvalue)
    (if (>= (`self.CurrentFadeTime`) (`self.FadeDuration`))
      (set `self.IsFading` false)
      (`self.K2_DestroyActor`))))

(fn `UserConstructionScript`)